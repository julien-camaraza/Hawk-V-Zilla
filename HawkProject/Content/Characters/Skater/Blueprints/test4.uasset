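; Test skater Blueprint that drives a physics-based skateboard from movement axis input.
; MoveForward input applies a force to the physics capsule along the skateboard mesh's forward vector, scaled by the axis value and Speed.
; MoveRight input is only stored in a variable, with no steering logic in this graph.
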(event EventBeginPlay)

(event Collision|EventActorBeginOverlap
  (params (OtherActor :type Actor%20Object%20Reference)))

(event EventTick
  (params (DeltaSeconds :type Float%20%28single-precision%29)))

(event Input|AxisEvents|InputAxisMoveRight
  (params (AxisValue :type Float%20%28single-precision%29))
  (Variables|Default|SetmoveRight AxisValue))

(event Input|AxisEvents|InputAxisMoveForward
  (params (AxisValue :type Float%20%28single-precision%29))
  (Variables|Default|SetmoveForward AxisValue)
  (Physics|AddForce (Variables|Default|GetphysicsCapsule) (* (Math|Vector|GetForwardVector (Variables|Default|GetskateboardMesh)) (* (Variables|Default|GetmoveForward) (Variables|Default|Getspeed))) "None" false))

(fn ConstructionScript)