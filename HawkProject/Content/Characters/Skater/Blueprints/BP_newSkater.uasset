(event Custom|crouchDeeper
  ;[1 1 1] When player presses down, begin crouching. The animation blends and jump height increases
  (Variables|Kickflip|SetcrouchAmount (Math|Float|Clamp(Float) (+ (Variables|Kickflip|GetcrouchAmount) 1.0) 0.0 1e+02)))

(event Custom|switchArm
  (bind _baseballbat (Variables|Default|GetbaseballBat))
  ;[1 1 1] Shooting
  ;;[1 1 1] When grabbing bat, attach it to hand and move it at the right angle. Reverse when putting it on back
  (Transformation|DetachFromComponent _baseballbat "KeepWorld" "KeepWorld" "KeepWorld" true)
  (Transformation|AttachComponentToComponent _baseballbat (Variables|Default|GetcharacterMesh) "hand_r" "SnapToTarget" "SnapToTarget" "KeepRelative" false)
  (Transformation|SetRelativeTransform _baseballbat (Variables|swingBat|GetarmBatTransform) false false))

(event Custom|aim
  (bind _followcamera (Variables|Default|GetFollowCamera))
  (bind _relativerotation (Variables|/Script/Engine.SceneComponent|GetRelativeRotation _followcamera))
  ;[1 1 1] Shooting
  ;;[1 1 1] When aiming: slow down the game, close the FOV a bit, and bring the camera closer to the player
  (bind (_direction _timedialation _fov _springarmlength _cameraheight) (Timeline|slowMo PlayFromStart)
    (:Update
      (Utilities|Time|SetGlobalTimeDilation _timedialation)
      (Camera|SetFieldOfView (Variables|Default|GetFollowCamera) _fov)
      (Variables|/Script/Engine.SpringArmComponent|SetTargetArmLength (Variables|Default|GetCameraBoom) _springarmlength)
      (Transformation|SetRelativeLocation _followcamera (Math|Vector|MakeVector (.roll _relativerotation) (.pitch _relativerotation) _cameraheight) false false))
    (:Finished
      (Variables|swingBat|SetshotReady true))))

(event Custom|rollingSound
  ;[1 1 1] Every second, call the cue for the board rolling against the ground
  (if (not (Variables|RailGrind|GetrailGrinding))
    (if (and (Variables|generalUse|GetonGround) (> (Class|WheeledVehicleMovementComponent|GetForwardSpeed (Variables|Default|GetVehicleMovement)) 0.0))
      (Audio|PlaySoundatLocation "/Game/Characters/Skater/Audio/A_Roll_Cue.A_Roll_Cue" (Transformation|GetWorldLocation (Variables|Character|GetMesh)) "0, 0, 0" 1.0 1.0 0.0 0 0 0))))

(event Custom|stopSwinging
  ;[1 1 1] Shooting
  ;;[1 1 1] Triggers sequence for aiming and shooting
  ;;;[1 1 1] Reset variables when shooting sequence is over
  (Variables|swingBat|Setswinging false)
  (Variables|swingBat|SetshotReady false)
  (Variables|swingBat|Setswung false))

(event Custom|returnCam
  (bind _followcamera (Variables|Default|GetFollowCamera))
  (bind _relativerotation (Variables|/Script/Engine.SceneComponent|GetRelativeRotation _followcamera))
  ;[1 1 1] Shooting
  ;;[1 1 1] Reset camera FOV and distance after shooting
  (bind (_direction _fov _armlength _cameraheight) (Timeline|returnCamera PlayFromStart)
    (:Update
      (Camera|SetFieldOfView (Variables|Default|GetFollowCamera) _fov)
      (Variables|/Script/Engine.SpringArmComponent|SetTargetArmLength (Variables|Default|GetCameraBoom) _armlength)
      (Transformation|SetRelativeLocation _followcamera (Math|Vector|MakeVector (.roll _relativerotation) (.pitch _relativerotation) _cameraheight) false false))))

(event Custom|restashBat
  (bind _baseballbat (Variables|Default|GetbaseballBat))
  ;[1 1 1] Shooting
  ;;[1 1 1] When grabbing bat, attach it to hand and move it at the right angle. Reverse when putting it on back
  (Transformation|DetachFromComponent (Variables|Default|GetbaseballBat) "KeepWorld" "KeepWorld" "KeepWorld" true)
  (Transformation|AttachComponentToComponent _baseballbat (Variables|Default|GetcharacterMesh) "spine_01" "SnapToTarget" "SnapToTarget" "KeepRelative" false)
  (Transformation|SetRelativeTransform _baseballbat (Variables|swingBat|GetbackBatTransform) false false))

(event Custom|grindSounds
  ;[1 1 1] Handles sounds for the railgrind
  (if (Variables|RailGrind|GetrailGrinding)
    (Audio|PlaySoundatLocation "/Game/Characters/Skater/Audio/A_Grind_Cue.A_Grind_Cue" (Transformation|GetWorldLocation (Variables|Character|GetMesh)) "0, 0, 0" 1.0 1.0 0.0 0 0 0)
    (else
      (Utilities|Time|ClearandInvalidateTimerbyHandle (Variables|RailGrind|GetgrindSoundsEvent)))))

(event Custom|chargeBall
  (Variables|Shooting|SetshotCharge (+ (Variables|Shooting|GetshotCharge) (Variables|Shooting|GetchargingSpeed))))

(event Game|Damage|EventAnyDamage
  (params (Damage :type Float%20%28single-precision%29) (DamageType :type Damage%20Type%20Object%20Reference) (InstigatedBy :type Controller%20Object%20Reference) (DamageCauser :type Actor%20Object%20Reference))
  (Development|PrintString (Utilities|String|ToString(Float) Damage)))

(event EventBeginPlay
  (Utilities|Time|SetTimerbyEvent (delegate Custom|chargeBall) 1.0 true)
  (Utilities|Time|SetTimerbyEvent (delegate Custom|rollingSound) 1.0 true)
  (Utilities|Time|SetTimerbyFunctionName self "checkOnGround" 0.01 true) ; Using 2 line traces, check if the player is on the ground
)

(event Input|ActionEvents|InputActionJump
  (params (Key :type Key%20Structure :default "None"))
  (bind _charactermesh (Variables|Default|GetcharacterMesh))
  (bind _relativelocation (Variables|/Script/Engine.SceneComponent|GetRelativeLocation _charactermesh))
  (:Pressed
    ;[1 1 1] When player presses down, begin crouching. The animation blends and jump height increases
    (Variables|Kickflip|Setcrouching true)
    (bind _returnvalue (Utilities|Time|SetTimerbyEvent (delegate Custom|crouchDeeper) 0.01 true))
    (Variables|Kickflip|SetcrouchDeeperEvent _returnvalue))
  (:Released
    ;[1 1 1] Stop crouching
    (Utilities|Time|ClearandInvalidateTimerbyHandle (Variables|Kickflip|GetcrouchDeeperEvent))
    ;[1 1 1] Jump based on how much player crouched with a 50% floor.
    (if (> (Variables|Kickflip|GetcrouchAmount) (Variables|Kickflip|GetmininumCrouchToJump))
      (Variables|Animation|Setjumping true)
      (Physics|AddImpulse (Variables|Character|GetMesh) (Math|Vector|MakeVector 0.0 0.0 5e+02) "None" true)
      (Components|Timeline|SetPlayRate (Variables|Default|GetkickflipTimeline) (/ 1.2 (/ (Math|Float|Clamp(Float) (Variables|Kickflip|GetcrouchAmount) 5e+01 1e+02) 1e+02)))
      (Audio|PlaySoundatLocation "/Game/Characters/Skater/Audio/A_Flip_Cue.A_Flip_Cue" (Transformation|GetWorldLocation (Variables|Character|GetMesh)) "0, 0, 0" 1.0 1.0 0.0 0 0 0)
      (bind _boardheight (Timeline|kickflipTimeline PlayFromStart)
        (:Update
          (Transformation|SetRelativeLocation _charactermesh (Math|Vector|MakeVector (.x _relativelocation) (.y _relativelocation) (Math|Float|Lerp 0.0 (* (/ (Math|Float|Clamp(Float) (Variables|Kickflip|GetcrouchAmount) 5e+01 1e+02) 1e+02) (Variables|Kickflip|GetmaxJumpHeight)) _boardheight)) false false))
        (:Finished
          (Utilities|FlowControl|Sequence
            (:then_0
              ;[1 1 1] Reset Variables
              (Variables|Kickflip|SetcrouchAmount 0.0 :!label _label)
              (Variables|Kickflip|Setcrouching false)
              (Variables|Animation|Setjumping false))
            (:then_1
              (Audio|PlaySoundatLocation "/Game/Characters/Skater/Audio/A_Flip_Cue.A_Flip_Cue" (Transformation|GetWorldLocation (Variables|Character|GetMesh)) "0, 0, 0" 1.0 1.0 0.0 0 0 0)))))
      (else
        (goto _label)))))

(event Input|ActionEvents|InputActionRailGrind
  (params (Key :type Key%20Structure :default "None"))
  (bind _currentrail (Variables|RailGrind|GetcurrentRail))
  (bind _mesh (Variables|Character|GetMesh))
  (bind _mesh_2 (Variables|Character|GetMesh))
  (bind _currentrail_2 (Variables|RailGrind|GetcurrentRail))
  (bind _spline (Variables|/Game/MapObjects/BP_rail.BP_rail_C|GetSpline _currentrail_2))
  (bind _spline_2 (Variables|/Game/MapObjects/BP_rail.BP_rail_C|GetSpline _currentrail))
  (:Pressed
    ;[1 1 1] Checks if already grinding + if there's a nearby rail
    (if (not (Variables|RailGrind|GetrailGrinding))
      (Utilities|IsValid (Variables|RailGrind|GetcurrentRail)
        (:Is%20Valid
          (Variables|RailGrind|SetrailGrinding true)
          ;[1 1 1] Store current velocity to give back to the player after grind
          (bind _returnvalue (Physics|GetPhysicsLinearVelocity _mesh "None"))
          (bind _output_get (Variables|RailGrind|SetcurrentVelocity _returnvalue))
          (Variables|RailGrind|SetcurrentRotation (Variables|/Script/Engine.SceneComponent|GetRelativeRotation _mesh)) ; Same for rotation
          ;[1 1 1] Edit speed of timeline based on character's speed and length of spline
          (Transformation|SetRelativeRotation (Variables|Character|GetMesh) (Spline|GetRotationatSplinePoint _spline 0 "Local") false true)
          (Components|Timeline|SetPlayRate (Variables|Default|GetrailGrind) (* (/ (Spline|GetSplineLength _spline) 3e+03) (/ (Math|Float|Clamp(Float) (Math|Vector|VectorLength _output_get) 2e+03 5e+03) 3e+03)))
          (Physics|SetPhysicsLinearVelocity (Variables|Character|GetMesh) "0, 0, 0" false "None") ; Stop player's current physics
          (bind _returnvalue_2 (Utilities|Time|SetTimerbyEvent (delegate Custom|grindSounds) 0.1 true))
          (Variables|RailGrind|SetgrindSoundsEvent _returnvalue_2)
          ;[1 1 1] Move player along rail
          (bind _newtrack_0 (Timeline|railGrind PlayFromStart)
            (:Update
              (Transformation|SetWorldLocation (Variables|Character|GetMesh) (Spline|GetLocationatDistanceAlongSpline _spline_2 (Math|Float|Lerp 0.0 (Spline|GetSplineLength _spline_2) _newtrack_0) "World") false true))
            (:Finished
              ;[1 1 1] Give back their momentum and reset the rail grind
              (Transformation|SetRelativeRotation _mesh_2 (Variables|RailGrind|GetcurrentRotation) false true)
              (Physics|SetPhysicsLinearVelocity _mesh_2 (Variables|RailGrind|GetcurrentVelocity) false "None")
              (Variables|RailGrind|SetrailGrinding false))))))))

(event Input|ActionEvents|InputActionShoot
  (params (Key :type Key%20Structure :default "None"))
  ;[1 1 1] Shooting
  ;;[1 1 1] Triggers sequence for aiming and shooting
  (:Pressed
    (if (Variables|swingBat|Getswinging)
      (if (Variables|swingBat|GetshotReady)
        (bind (_out_hit_location _out_hit_hit_actor) (CallFunction|ShootfromCamera))
        (Variables|Shooting|SetballCurrentLocation (Transformation|GetWorldLocation (Variables|Default|Getbaseball)))
        (Variables|Shooting|SetballGoTo _out_hit_location)
        (Variables|swingBat|Setswung true)
        (bind (_direction _newtrack_0 _baseballlocation) (Timeline|stopSlowMo PlayFromStart)
          (:Update
            (Utilities|Time|SetGlobalTimeDilation _newtrack_0)
            (Transformation|SetWorldLocation (Variables|Default|Getbaseball) (Math|Vector|Lerp(Vector) (Variables|Shooting|GetballCurrentLocation) (Variables|Shooting|GetballGoTo) _baseballlocation) false false))
          (:Finished
            (bind _asbp_kaiju_parent (Utilities|Casting|CastToBP_kaijuParent _out_hit_hit_actor))
            (Game|Damage|ApplyDamage _asbp_kaiju_parent 1e+01 0 0)
            (Transformation|AttachComponentToComponent (Variables|Default|Getbaseball) (Variables|Default|GetbaseballBat) "None" "SnapToTarget" "SnapToTarget" "SnapToTarget" true)
            (Transformation|SetRelativeLocation (Variables|Default|Getbaseball) (Variables|Shooting|GetballRelativeLocation) false false)
            (Components|Activation|Deactivate (Variables|Default|GetNiagara)))
          (:PlaySound
            (Components|Activation|Activate (Variables|Default|GetNiagara) false)
            (Audio|PlaySoundatLocation "/Game/Characters/Skater/Audio/A_SwingBat_Cue.A_SwingBat_Cue" (Transformation|GetWorldLocation (Variables|Default|GetbaseballBat)) "0, 0, 0" 1.0 1.0 0.0 0 0 0)
            (Transformation|DetachFromComponent (Variables|Default|Getbaseball) "KeepWorld" "KeepWorld" "KeepWorld" true))))
      (else
        (Variables|swingBat|Setswinging true)))))

(event Input|AxisEvents|InputAxisMoveForward
  (params (AxisValue :type Float%20%28single-precision%29))
  (if (not (Variables|RailGrind|GetrailGrinding))
    ;[1 1 1] Calculate how often to kick
    (if (> AxisValue 0.0)
      (if (< (Variables|Animation|GetkickTimer) (Variables|Animation|GettimeKicking))
        (Variables|Animation|SetkickTimer (Math|Float|Clamp(Float) (+ (Variables|Animation|GetkickTimer) 1.0) 0.0 (Variables|Animation|GettimeKicking)))
        (if (Variables|Kickflip|Getcrouching)
          (Variables|Default|Setaccelerating false)
          (else
            (Variables|Default|Setaccelerating true)))
        (else
          (Variables|Default|Setaccelerating false)
          (bind _output_get (Variables|Animation|SetkickWait (Math|Float|Clamp(Float) (+ (Variables|Animation|GetkickWait) 1.0) 0.0 (Variables|Animation|GettimeBetweenKicks))))
          (if (< _output_get (Variables|Animation|GettimeBetweenKicks))
            _
            (else
              (Variables|Animation|SetkickWait 0.0)
              (Variables|Animation|SetkickTimer 0.0)))))
      (Class|WheeledVehicleMovementComponent|SetThrottleInput (Variables|Default|GetVehicleMovement) AxisValue)
      (else
        (Variables|Default|Setaccelerating false)
        (Variables|Animation|SetkickTimer 0.0)))))

(event Input|AxisEvents|InputAxisMoveRight
  (params (AxisValue :type Float%20%28single-precision%29))
  ;[1 1 1] Steering
  (Class|WheeledVehicleMovementComponent|SetSteeringInput (Variables|Default|GetVehicleMovement) AxisValue))

(event Input|AxisEvents|InputAxisLookUp
  (params (AxisValue :type Float%20%28single-precision%29))
  (bind _cameraboom (Variables|Default|GetCameraBoom))
  (bind _relativerotation (Variables|/Script/Engine.SceneComponent|GetRelativeRotation _cameraboom))
  ;[1 1 1] Camera Controls
  (Transformation|SetRelativeRotation (Variables|Default|GetCameraBoom) (Math|Rotator|MakeRotator 0.0 (Math|Float|Clamp(Float) (+ (* -1 (* AxisValue (Class|GameplayStatics|GetGlobalTimeDilation))) (.pitch _relativerotation)) -25.0 1e+01) (Math|Float|Clamp(Float) (+ (.yaw _relativerotation) (* (stale Input|AxisEvents|InputAxisLookRight AxisValue) (Class|GameplayStatics|GetGlobalTimeDilation))) -1.1e+02 1.1e+02)) false false))

(event Input|AxisEvents|InputAxisLookRight
  (params (AxisValue :type Float%20%28single-precision%29))
  (bind _cameraboom (Variables|Default|GetCameraBoom))
  (bind _relativerotation (Variables|/Script/Engine.SceneComponent|GetRelativeRotation _cameraboom))
  ;[1 1 1] Camera Controls
  (Transformation|SetRelativeRotation (Variables|Default|GetCameraBoom) (Math|Rotator|MakeRotator 0.0 (Math|Float|Clamp(Float) (+ (* -1 (* (stale Input|AxisEvents|InputAxisLookUp AxisValue) (Class|GameplayStatics|GetGlobalTimeDilation))) (.pitch _relativerotation)) -25.0 1e+01) (Math|Float|Clamp(Float) (+ (.yaw _relativerotation) (* AxisValue (Class|GameplayStatics|GetGlobalTimeDilation))) -1.1e+02 1.1e+02)) false false))

(fn ConstructionScript
  (Transformation|SetRelativeTransform (Variables|Default|GetCameraBoom) (Math|Transform|MakeTransform "0, 0,180.000000" "-10.000000, 0,0.000000" "1,1,1") false false)
  (Components|Timeline|SetPlayRate (Variables|Default|GetslowMo) 2.0)
  (Components|Timeline|SetPlayRate (Variables|Default|GetstopSlowMo) 2.0)
  (Variables|Shooting|SetballRelativeLocation (Variables|/Script/Engine.SceneComponent|GetRelativeLocation (Variables|Default|Getbaseball))))

(fn CheckonGround
  (bind _fronttrace (Variables|Default|GetfrontTrace))
  (bind _backtrace (Variables|Default|GetbackTrace))
  (bind _returnvalue (Transformation|GetWorldLocation _backtrace))
  (bind _returnvalue_2 (Transformation|GetWorldLocation _fronttrace))
  (bind (_x _y _z) (Math|Vector|BreakVector _returnvalue))
  (bind (_x_2 _y_2 _z_2) (Math|Vector|BreakVector _returnvalue_2))
  (bind _returnvalue_3 (Collision|LineTraceByChannel _returnvalue_2 (Math|Vector|MakeVector _x_2 _y_2 (- _z_2 (Variables|generalUse|GetskateboardHeight))) "TraceTypeQuery1" false 0 "ForDuration"))
  (bind _returnvalue_4 (Collision|LineTraceByChannel _returnvalue (Math|Vector|MakeVector _x _y (- _z (Variables|generalUse|GetskateboardHeight))) "TraceTypeQuery1" false 0 "ForDuration"))
  (if (and _returnvalue_3 _returnvalue_4)
    (Variables|generalUse|SetonGround true)
    (else
      (Variables|generalUse|SetonGround false))))

(fn ShootfromCamera
  (bind _followcamera (Variables|Default|GetFollowCamera))
  (bind _returnvalue (Transformation|GetWorldLocation _followcamera))
  (bind _outhit (Collision|LineTraceForObjects _returnvalue (+ _returnvalue (* (Math|Vector|GetForwardVector _followcamera) (Variables|shooting|GetshotLength))) (Variables|shooting|GetshootableObjects) false 0 "None"))
  (return (.location _outhit) (.hitactor _outhit)))