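; Kaiju shockwave actor that raises a trail of mesh instances along the AttackLine spline, one point after another, starting on BeginPlay.
; Each step adds a Hierarchical Instanced Static Mesh instance at the next spline point, and the Grow timeline animates its Z scale up from zero.
; Target height ramps up over the first few instances to full scale, and each timeline finish triggers the next point until the spline ends.
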(event EventTick
  (params (DeltaSeconds :type Float%20%28single-precision%29)))

(event EventBeginPlay
  (bind _hierarchicalinstancedstaticmesh (Variables|Default|GetHierarchicalInstancedStaticMesh))
  (if (< (Variables|Default|GetincrementShockCount) (Spline|GetNumberOfSplinePoints (Variables|Default|GetattackLine))) :!label _label
    (Components|InstancedStaticMesh|AddInstance (Variables|Default|GetHierarchicalInstancedStaticMesh) (Spline|GetTransformatSplinePoint (Variables|Default|GetattackLine) (Variables|Default|GetincrementShockCount) "Local" false))
    (bind _newtrack_0 (Timeline|grow PlayFromStart)
      (:Update
        (Components|InstancedStaticMesh|UpdateInstanceTransform _hierarchicalinstancedstaticmesh (Variables|Default|GetincrementShockCount) (Math|Transform|MakeTransform (.location (.OutInstanceTransform (Components|InstancedStaticMesh|GetInstanceTransform _hierarchicalinstancedstaticmesh (Variables|Default|GetincrementShockCount) false))) (.rotation (.OutInstanceTransform (Components|InstancedStaticMesh|GetInstanceTransform _hierarchicalinstancedstaticmesh (Variables|Default|GetincrementShockCount) false))) (Math|Vector|MakeVector (.x (.scale (.OutInstanceTransform (Components|InstancedStaticMesh|GetInstanceTransform _hierarchicalinstancedstaticmesh (Variables|Default|GetincrementShockCount) false)))) (.y (.scale (.OutInstanceTransform (Components|InstancedStaticMesh|GetInstanceTransform _hierarchicalinstancedstaticmesh (Variables|Default|GetincrementShockCount) false)))) (Math|Float|Lerp 0.0 (* (Math|Integer|Clamp(Integer) (Variables|Default|GetincrementShockCount) 1 4) 0.25) _newtrack_0))) false false false))
      (:Finished
        (Variables|Default|SetincrementShockCount (Math|Integer|Clamp(Integer) (+ (Variables|Default|GetincrementShockCount) 1) 0 (Spline|GetNumberOfSplinePoints (Variables|Default|GetattackLine))))
        (goto _label)))))

(fn ConstructionScript)