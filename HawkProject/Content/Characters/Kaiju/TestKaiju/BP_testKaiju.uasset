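; BP_testKaiju is a test kaiju Blueprint that adds a roar and a shockwave attack to its parent class.
; Roar plays a sound at SoundSpawn.
; summonShockwave spawns and triggers a BP_shockwave at ShockwaveSpawn, shakes the screen through coreGameMode and plays a rumble there.
; The construction script sets HandBoneName to a right-hand thumb bone before running the parent's script.
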(event Custom|summonShockwave
  (bind _shockwavespawn (Variables|Default|GetshockwaveSpawn))
  (bind _returnvalue (Transformation|GetWorldTransform _shockwavespawn))
  (bind _returnvalue_2 (Game|SpawnActorfromClass "/Game/Characters/Kaiju/Shared/BP_shockwave.BP_shockwave_C" (Math|Transform|MakeTransform (.location _returnvalue) (.rotation _returnvalue) "1,1,1") "Undefined" 0 0))
  (Default|Spawn _returnvalue_2)
  (Default|ShakeScreen (.AsCore%20Game%20Mode (Utilities|Casting|CastTocoreGameMode (Game|GetGameMode))) (.location _returnvalue))
  (Audio|PlaySoundatLocation "/Game/Core/Audio/City/A_rumble1_Cue.A_rumble1_Cue" (.location _returnvalue) "0, 0, 0" 1.0 1.0 0.0 0 0 0))

(event EventBeginPlay
  (|CallParentFunction))

(event Collision|EventActorBeginOverlap
  (params (OtherActor :type Actor%20Object%20Reference))
  (|CallParentFunction OtherActor) ; This node is disabled and will not be called.\nDrag off pins to build functionality.
)

(event EventTick
  (params (DeltaSeconds :type Float%20%28single-precision%29))
  (|CallParentFunction DeltaSeconds) ; This node is disabled and will not be called.\nDrag off pins to build functionality.
)

(event EventRoar
  (Audio|PlaySoundatLocation "/Game/Characters/Kaiju/TestKaiju/Audio/A_roar_CUE.A_roar_CUE" (Transformation|GetWorldLocation (Variables|Default|GetsoundSpawn)) "0, 0, 0" 1.0 1.0 0.0 0 0 0))

(fn ConstructionScript
  (Variables|Default|SethandBoneName "RightHandThumb4")
  (|CallParentFunction))