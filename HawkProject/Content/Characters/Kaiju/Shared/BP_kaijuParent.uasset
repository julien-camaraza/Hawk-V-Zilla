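; Shared parent Blueprint for kaiju bosses that topple buildings and throw rubble at the skater player.
; Health thresholds advance phases on AIC_testKaiju, failing the current task and blending in a hit reaction.
; Timelines drive 90-degree turns and player-facing rotation; compass direction selects which cached buildings can fall.
; Action events report through CurrentTask; rubble spawns on the hand socket mid-turn and is later launched near the player.
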(event Custom|rotate90Degrees
  (params (Negative :type Boolean))
  ;[1 1 1] Rotates character 90 degrees, no animation yet
  (Variables|propertyTracking|SetcurrentRelativeRotation (Variables|/Script/Engine.SceneComponent|GetRelativeRotation (Variables|Collision|GetCapsuleComponent)))
  (if Negative
    (CallFunction|SwitchDirection true)
    (Variables|propertyTracking|SetrotationToGoTo (Math|Rotator|MakeRotator (.roll (Variables|propertyTracking|GetcurrentRelativeRotation)) (.pitch (Variables|propertyTracking|GetcurrentRelativeRotation)) (- (.yaw (Variables|propertyTracking|GetcurrentRelativeRotation)) 9e+01)))
    (bind _rotation (Timeline|rotate PlayFromStart)
      (:Update
        (Transformation|SetRelativeRotation (Variables|Collision|GetCapsuleComponent) (Math|Rotator|Lerp(Rotator) (Variables|propertyTracking|GetcurrentRelativeRotation) (Variables|propertyTracking|GetrotationToGoTo) _rotation) false false))
      (:Finished
        (CallFunction|TaskFinished true)))
    (else
      (CallFunction|SwitchDirection false)
      (Variables|propertyTracking|SetrotationToGoTo (Math|Rotator|MakeRotator (.roll (Variables|propertyTracking|GetcurrentRelativeRotation)) (.pitch (Variables|propertyTracking|GetcurrentRelativeRotation)) (+ (.yaw (Variables|propertyTracking|GetcurrentRelativeRotation)) 9e+01)))
      (Timeline|rotate PlayFromStart))))

(event Custom|taskFinished
  (params (Success :type Boolean))
  ;[1 1 1] Move on to next AI event
  (AI|BehaviorTree|FinishExecute (Variables|AI|GetcurrentTask) Success))

(event Custom|taskFailed
  (AI|BehaviorTree|FinishExecute (Variables|AI|GetcurrentTask))
  (Variables|Animation|SetcurrentAction "NewEnumerator2"))

(event Custom|DestroyBuilding
  ;[1 1 1] When destroying a building, start the animation, wait, then choose a standing building in front of the monster to topple
  (Variables|Animation|SetcurrentAction "NewEnumerator0")
  (Utilities|FlowControl|Delay 1.0)
  (switch Utilities|FlowControl|Switch|SwitchonEBuildingLocation (Variables|AI|GetcurrentDirection)
    (:NewEnumerator0
      (Utilities|ChooseBuildingtoDestroy (Variables|CityInteraction|GetnorthBuildings)))
    (:NewEnumerator1
      (Utilities|ChooseBuildingtoDestroy (Variables|CityInteraction|GetsouthBuildings)))
    (:NewEnumerator2
      (Utilities|ChooseBuildingtoDestroy (Variables|CityInteraction|GeteastBuildings)))
    (:NewEnumerator3
      (Utilities|ChooseBuildingtoDestroy (Variables|CityInteraction|GetwestBuildings)))))

(event Custom|incrementPhase
  ;[1 1 1] Increment phase by 1 and tell the AI controller
  (bind _result (Math|Integer|IncrementInt (Variables|propertyTracking|GetcurrentPhase))
    (:%20%20
      (bind _asaic_test_kaiju (Utilities|Casting|CastToAIC_testKaiju (Pawn|GetController)))
      (Variables|/Game/AI/testKaiju/AIC_testKaiju.AIC_testKaiju_C|Setphase _asaic_test_kaiju _result))))

(event Custom|throwRubble
  (Variables|Animation|SetcurrentAction "NewEnumerator1")
  (CallFunction|LookatPlayerEvent))

(event Custom|throwRock
  (bind _rubble (Variables|Default|Getrubble))
  (bind _playercharacter (Variables|Default|GetplayerCharacter))
  (bind _mesh (Variables|/Script/PhysXVehicles.WheeledVehicle|GetMesh _playercharacter))
  (bind _returnvalue (Transformation|GetWorldLocation _mesh))
  ;[1 1 1] Detatch from kaiju and begin event in rubble that throws towards player
  (Transformation|DetachFromActor _rubble "KeepWorld" "KeepRelative" "KeepWorld")
  (Default|FlyTowardsPlayer _rubble (Math|Vector|MakeVector (+ (Math|Random|RandomFloatinRange 2e+03 3e+03) (.x _returnvalue)) (+ (.y _returnvalue) (Math|Random|RandomFloatinRange 2e+03 3e+03)) (.z _returnvalue)) self))

(event Custom|attack1
  (Variables|Animation|SetcurrentAction "NewEnumerator3")
  (CallFunction|LookatPlayerEvent))

(event Custom|lookAtPlayerEvent
  ;[1 1 1] Rotate torwards player
  (CallFunction|GetLookatPlayer)
  (Components|Timeline|SetPlayRate (Variables|Default|GetlookAtPlayer) (/ 75.0 (Math|Float|Absolute(Float) (- (Math|Float|Absolute(Float) (.yaw (Variables|propertyTracking|GetrotationToGoTo))) (Math|Float|Absolute(Float) (.yaw (Variables|propertyTracking|GetcurrentRelativeRotation)))))))
  (bind _rotatetowardsplayer (Timeline|lookAtPlayer PlayFromStart)
    (:Update
      (Transformation|SetRelativeRotation (Variables|Collision|GetCapsuleComponent) (Math|Rotator|Lerp(Rotator) (Variables|propertyTracking|GetcurrentRelativeRotation) (Variables|propertyTracking|GetrotationToGoTo) _rotatetowardsplayer) false false))
    (:NewTrack_1
      (switch Utilities|FlowControl|Switch|SwitchonE_kaijuMoves (Variables|Animation|GetcurrentAction)
        (:NewEnumerator1
          ;[1 1 1] Play pickup animation and spawn rubble in hand
          (bind _returnvalue (Game|SpawnActorfromClass "/Game/Core/BP_rubble.BP_rubble_C" (Math|Transform|MakeTransform (Transformation|GetWorldLocation (Variables|Default|GetrubbleSpawn)) "0, 0, 0" "10.000000,10.000000,10.000000") "Undefined" 0 0))
          (bind _output_get (Variables|Default|Setrubble _returnvalue))
          (Transformation|AttachComponentToComponent _output_get (Variables|Default|GetrubbleSpawn) "None" "SnapToTarget" "SnapToTarget" "KeepWorld" true))))))

(event Custom|goToPreviousRotation
  ;[1 1 1] Rotate torwards player
  (bind _rotatetowardsplayer (Timeline|lookAtPlayer ReverseFromEnd)
    (:Update
      (Transformation|SetRelativeRotation (Variables|Collision|GetCapsuleComponent) (Math|Rotator|Lerp(Rotator) (Variables|propertyTracking|GetcurrentRelativeRotation) (Variables|propertyTracking|GetrotationToGoTo) _rotatetowardsplayer) false false))
    (:NewTrack_1
      (switch Utilities|FlowControl|Switch|SwitchonE_kaijuMoves (Variables|Animation|GetcurrentAction)
        (:NewEnumerator1
          ;[1 1 1] Play pickup animation and spawn rubble in hand
          (bind _returnvalue (Game|SpawnActorfromClass "/Game/Core/BP_rubble.BP_rubble_C" (Math|Transform|MakeTransform (Transformation|GetWorldLocation (Variables|Default|GetrubbleSpawn)) "0, 0, 0" "10.000000,10.000000,10.000000") "Undefined" 0 0))
          (bind _output_get (Variables|Default|Setrubble _returnvalue))
          (Transformation|AttachComponentToComponent _output_get (Variables|Default|GetrubbleSpawn) "None" "SnapToTarget" "SnapToTarget" "KeepWorld" true))))))

(event EventBeginPlay
  (CallFunction|StoreBuildings) ; add all buildings to the approrpirate array for referencing
  (CallFunction|IncrementPhase)
  (Variables|Default|SetplayerCharacter (.AsBP%20New%20Skater (Utilities|Casting|CastToBP_newSkater (Game|Player|GetPlayerPawn 0)))))

(event Game|Damage|EventAnyDamage
  (params (Damage :type Float%20%28single-precision%29) (DamageType :type Damage%20Type%20Object%20Reference) (InstigatedBy :type Controller%20Object%20Reference) (DamageCauser :type Actor%20Object%20Reference))
  (bind _output_get (Variables|propertyTracking|SetHealth (- (Variables|propertyTracking|GetHealth) Damage)))
  (Development|PrintString (Utilities|String|ToString(Text) (Utilities|Text|FormatText "Health Remaining: {0}" _output_get)))
  (switch int (Variables|propertyTracking|GetcurrentPhase)
    (:1
      (if (<= (Variables|propertyTracking|GetHealth) (Variables|AI|Getphase2Health))
        (CallFunction|IncrementPhase)
        (CallFunction|TaskFailed :!label _label)
        (bind _blendstate (Timeline|blendToHit PlayFromStart)
          (:Update
            (Variables|Default|SethitBlend _blendstate)))))
    (:2
      (if (<= (Variables|propertyTracking|GetHealth) (Variables|AI|Getphase3Health))
        (CallFunction|IncrementPhase)
        (goto _label)))))

(fn ConstructionScript
  (Transformation|AttachComponentToComponent (Variables|Default|GetrubbleSpawn) (Variables|Character|GetMesh) (Variables|CityInteraction|GethandBoneName) "SnapToTarget" "SnapToTarget" "KeepRelative" true))

(fn StoreBuildings
  ;[1 1 1] add all buildings to the approrpirate array for referencing
  (bind _outactors (Actor|GetAllActorsOfClass "/Game/Core/BP_building.BP_building_C"))
  (for _array_element _outactors
    (switch Utilities|FlowControl|Switch|SwitchonEBuildingLocation (Variables|/Game/Core/BP_building.BP_building_C|GetbuildingDirection _array_element)
      (:NewEnumerator0
        (Utilities|Array|AddUnique (Variables|CityInteraction|GetnorthBuildings) _array_element))
      (:NewEnumerator1
        (Utilities|Array|AddUnique (Variables|CityInteraction|GetsouthBuildings) _array_element))
      (:NewEnumerator2
        (Utilities|Array|AddUnique (Variables|CityInteraction|GeteastBuildings) _array_element))
      (:NewEnumerator3
        (Utilities|Array|AddUnique (Variables|CityInteraction|GetwestBuildings) _array_element)))))

(fn SwitchDirection
  (params (Negative :type Boolean))
  ;[1 1 1] Update direction tracker when rotating
  (if Negative
    (switch Utilities|FlowControl|Switch|SwitchonEBuildingLocation (Variables|AI|GetcurrentDirection)
      (:NewEnumerator0
        (Variables|AI|SetcurrentDirection "NewEnumerator3"))
      (:NewEnumerator1
        (Variables|AI|SetcurrentDirection "NewEnumerator2"))
      (:NewEnumerator2
        (Variables|AI|SetcurrentDirection "NewEnumerator0"))
      (:NewEnumerator3
        (Variables|AI|SetcurrentDirection "NewEnumerator1")))
    (else
      (switch Utilities|FlowControl|Switch|SwitchonEBuildingLocation (Variables|AI|GetcurrentDirection)
        (:NewEnumerator0
          (Variables|AI|SetcurrentDirection "NewEnumerator2"))
        (:NewEnumerator1
          (Variables|AI|SetcurrentDirection "NewEnumerator3"))
        (:NewEnumerator2
          (Variables|AI|SetcurrentDirection "NewEnumerator1"))
        (:NewEnumerator3
          (Variables|AI|SetcurrentDirection "NewEnumerator0"))))))

(fn GetLookatPlayer
  (Variables|propertyTracking|SetcurrentRelativeRotation (Variables|/Script/Engine.SceneComponent|GetRelativeRotation (Variables|Collision|GetCapsuleComponent)))
  (Variables|propertyTracking|SetrotationToGoTo (Math|Rotator|FindLookatRotation (Transformation|GetWorldLocation (Variables|Collision|GetCapsuleComponent)) (Transformation|GetWorldLocation (Variables|/Script/PhysXVehicles.WheeledVehicle|GetMesh (Variables|Default|GetplayerCharacter))))))