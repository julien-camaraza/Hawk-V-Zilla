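; Kaiju shockwave attack that raises a row of meshes one after another along the AttackLine spline.
; The spawn event adds a hierarchical instanced mesh at each spline point and asks coreGameMode to shake the screen with that point's local location.
; The sped-up Grow timeline lerps the instance's Z scale up, taller for later points up to a cap.
; When it finishes, the counter increments and the loop repeats until points run out.
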(event Custom|spawn
  (bind _hierarchicalinstancedstaticmesh (Variables|Default|GetHierarchicalInstancedStaticMesh))
  ;[1 1 1] Check if there's remaining spline points
  (if (< (Variables|Default|GetincrementShockCount) (Spline|GetNumberOfSplinePoints (Variables|Default|GetattackLine))) :!label _label
    ;[1 1 1] If there is, summon a new instance of the mesh
    (Components|InstancedStaticMesh|AddInstance (Variables|Default|GetHierarchicalInstancedStaticMesh) (Spline|GetTransformatSplinePoint (Variables|Default|GetattackLine) (Variables|Default|GetincrementShockCount) "Local" false))
    (Default|ShakeScreen (.AsCore%20Game%20Mode (Utilities|Casting|CastTocoreGameMode (Game|GetGameMode))) (.Location (Math|Transform|BreakTransform (Spline|GetTransformatSplinePoint (Variables|Default|GetattackLine) (Variables|Default|GetincrementShockCount) "Local" false))))
    ;[1 1 1] Grow mesh
    (bind _newtrack_0 (Timeline|grow PlayFromStart)
      (:Update
        (Components|InstancedStaticMesh|UpdateInstanceTransform _hierarchicalinstancedstaticmesh (Variables|Default|GetincrementShockCount) (Math|Transform|MakeTransform (.location (.OutInstanceTransform (Components|InstancedStaticMesh|GetInstanceTransform _hierarchicalinstancedstaticmesh (Variables|Default|GetincrementShockCount) false))) (.rotation (.OutInstanceTransform (Components|InstancedStaticMesh|GetInstanceTransform _hierarchicalinstancedstaticmesh (Variables|Default|GetincrementShockCount) false))) (Math|Vector|MakeVector (.x (.scale (.OutInstanceTransform (Components|InstancedStaticMesh|GetInstanceTransform _hierarchicalinstancedstaticmesh (Variables|Default|GetincrementShockCount) false)))) (.y (.scale (.OutInstanceTransform (Components|InstancedStaticMesh|GetInstanceTransform _hierarchicalinstancedstaticmesh (Variables|Default|GetincrementShockCount) false)))) (Math|Float|Lerp 0.0 (* (Math|Integer|Clamp(Integer) (Variables|Default|GetincrementShockCount) 1 4) 0.25) _newtrack_0))) false false false))
      (:Finished
        ;[1 1 1] Increment counter
        (Variables|Default|SetincrementShockCount (Math|Integer|Clamp(Integer) (+ (Variables|Default|GetincrementShockCount) 1) 0 (Spline|GetNumberOfSplinePoints (Variables|Default|GetattackLine))))
        (goto _label)))))

(event EventTick
  (params (DeltaSeconds :type Float%20%28single-precision%29)))

(fn ConstructionScript
  (Components|Timeline|SetPlayRate (Variables|Default|Getgrow) 3.0))