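; BP_rail is a map rail that tells BP_newSkater which rail it is currently at.
; When the skater's HitboxCapsule enters the DetectionBox, the rail sets itself as that skater's CurrentRail.
; When that capsule leaves, it clears CurrentRail to None without checking which rail is stored, and both handlers print the value's display name for debugging.
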(event OnComponentBeginOverlap(detectionBox)
  (params (OverlappedComponent :type Primitive%20Component%20Object%20Reference) (OtherActor :type Actor%20Object%20Reference) (OtherComp :type Primitive%20Component%20Object%20Reference) (OtherBodyIndex :type Integer) (bFromSweep :type Boolean) (SweepResult :type Hit%20Result%20Structure%20%28by%20ref%29))
  (bind _asbp_new_skater (Utilities|Casting|CastToBP_newSkater OtherActor))
  (if (== OtherComp (Variables|/Script/HawkProject.C_newSkateboard|GethitboxCapsule _asbp_new_skater))
    (bind _output_get (Variables|/Game/Characters/Skater/Blueprints/BP_newSkater.BP_newSkater_C|SetcurrentRail _asbp_new_skater self))
    (Development|PrintString (Utilities|GetDisplayName _output_get))))

(event OnComponentEndOverlap(detectionBox)
  (params (OverlappedComponent :type Primitive%20Component%20Object%20Reference) (OtherActor :type Actor%20Object%20Reference) (OtherComp :type Primitive%20Component%20Object%20Reference) (OtherBodyIndex :type Integer))
  (bind _asbp_new_skater (Utilities|Casting|CastToBP_newSkater OtherActor))
  (if (== OtherComp (Variables|/Script/HawkProject.C_newSkateboard|GethitboxCapsule _asbp_new_skater))
    (bind _output_get (Variables|/Game/Characters/Skater/Blueprints/BP_newSkater.BP_newSkater_C|SetcurrentRail _asbp_new_skater 0))
    (Development|PrintString (Utilities|GetDisplayName _output_get))))

(event EventBeginPlay)

(event Collision|EventActorBeginOverlap
  (params (OtherActor :type Actor%20Object%20Reference)))

(event EventTick
  (params (DeltaSeconds :type Float%20%28single-precision%29)))

(fn ConstructionScript)