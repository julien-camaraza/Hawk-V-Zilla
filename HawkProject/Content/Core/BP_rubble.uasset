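; Rubble projectile that a Kaiju sends flying at a target location, damaging the skater it overlaps.
; On launch it spawns a red, glowing warning indicator with the rubble's mesh at the target, then a timeline lerps it there without sweeping.
; On arrival it removes the indicator, switches to blocking physics-only collision and tells the Kaiju the task is finished.
; Overlapping the skater applies damage and turns off the rubble's collision.
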(event OnComponentBeginOverlap(rubbleModel)
  (params (OverlappedComponent :type Primitive%20Component%20Object%20Reference) (OtherActor :type Actor%20Object%20Reference) (OtherComp :type Primitive%20Component%20Object%20Reference) (OtherBodyIndex :type Integer) (bFromSweep :type Boolean) (SweepResult :type Hit%20Result%20Structure%20%28by%20ref%29))
  (bind _rubblemodel (Variables|Default|GetrubbleModel))
  (bind _asbp_new_skater (Utilities|Casting|CastToBP_newSkater OtherActor))
  (Game|Damage|ApplyDamage _asbp_new_skater 1e+01 0 0)
  (Collision|SetCollisionEnabled _rubblemodel "NoCollision")
  (Collision|SetCollisionResponsetoAllChannels _rubblemodel "ECR_Ignore"))

(event Custom|flyTowardsPlayer
  (params (goToLocation :type Vector) (kaiju :type BP%20Kaiju%20Parent%20Object%20Reference))
  (bind _defaultsceneroot (Variables|Default|GetDefaultSceneRoot))
  (bind _rubblemodel (Variables|Default|GetrubbleModel))
  (Variables|Default|SetKaiju kaiju)
  (Variables|Default|SetcurrentWorldLocation (Transformation|GetWorldLocation _defaultsceneroot))
  (bind _returnvalue (Game|SpawnActorfromClass "/Game/Core/BP_warningIndicator.BP_warningIndicator_C" (Math|Transform|MakeTransform goToLocation "0, 0, 0" (Transformation|GetWorldScale _defaultsceneroot)) "Undefined" 0 0))
  (Default|Spawn _returnvalue (Variables|/Script/Engine.StaticMeshComponent|GetStaticMesh (Variables|Default|GetrubbleModel)) "(R=0.731771,G=0.156213,B=0.163492,A=1.000000)" 2.0)
  (bind _fly (Timeline|fly PlayFromStart)
    (:Update
      (Transformation|SetWorldLocation (Variables|Default|GetDefaultSceneRoot) (Math|Vector|Lerp(Vector) (Variables|Default|GetcurrentWorldLocation) goToLocation _fly) false false))
    (:Finished
      (Actor|DestroyActor _returnvalue)
      (Collision|SetCollisionEnabled _rubblemodel "PhysicsOnly")
      (Collision|SetCollisionResponsetoAllChannels _rubblemodel "ECR_Block")
      (Default|TaskFinished (Variables|Default|GetKaiju) true))))

(event EventBeginPlay)

(event Collision|EventActorBeginOverlap
  (params (OtherActor :type Actor%20Object%20Reference)))

(event EventTick
  (params (DeltaSeconds :type Float%20%28single-precision%29)))

(fn ConstructionScript)