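; BP_building is a building actor that a monster can knock over.
; The construction script toggles a forward-direction arrow, caches standing and fallen rotations 90 degrees of pitch apart, and sets the fall timeline's play rate.
; The fallOver event plays that timeline to lerp the mesh rotation, then clears Standing and tells the calling Monster its task finished.
; Random mesh scaling is present but disconnected.
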(event Custom|fallOver
  (params (monster :type BP%20Kaiju%20Parent%20Object%20Reference))
  (Variables|MonsterInteraction|SetMonster monster)
  (bind _lerprotation (Timeline|buildingFall PlayFromStart)
    (:Update
      (Transformation|SetRelativeRotation (Variables|Default|GetbuildingMesh) (Math|Rotator|Lerp(Rotator) (Variables|MonsterInteraction|GetstartingRotation) (Variables|MonsterInteraction|GetfallenRotation) _lerprotation) false false))
    (:Finished
      (Variables|MonsterInteraction|Setstanding false)
      (Default|TaskFinished (Variables|MonsterInteraction|GetMonster) true))))

(event EventBeginPlay)

(fn ConstructionScript
  (Utilities|FlowControl|Sequence
    (:then_1
      ;[1 1 1] Quickly choose if you want to see arrows indicating forward direction or not
      (Rendering|SetVisibility (Variables|Default|GetArrow) (Variables|Constructor|GetshowArrow?) false))
    (:then_2
      ;[1 1 1] Rotations to lerp between when falling
      (bind _output_get (Variables|MonsterInteraction|SetstartingRotation (Variables|/Script/Engine.SceneComponent|GetRelativeRotation (Variables|Default|GetbuildingMesh))))
      (Variables|MonsterInteraction|SetfallenRotation (Math|Rotator|MakeRotator (.roll _output_get) (- (.pitch _output_get) 9e+01) (.yaw _output_get))))
    (:then_3
      (Components|Timeline|SetPlayRate (Variables|Default|GetbuildingFall) (Variables|Default|GetfallSpeed)))))