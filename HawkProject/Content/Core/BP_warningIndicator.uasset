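; BP_warningIndicator is an actor that shows a tinted warning marker made of a static mesh and a decal.
; On BeginPlay it creates dynamic material instances for both, using M_3DIndicator_Inst for the mesh, and stores them.
; Its spawn event sets the mesh and pushes a color and emissive amount to both materials, so the caller defines the indicator's look.
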(event Custom|spawn
  (params (mesh :type Static%20Mesh%20Object%20Reference) (Color :type Linear%20Color%20Structure) (EmmisiveAmount :type Float%20%28single-precision%29))
  ;[1 1 1] Create the look of the material
  (Components|StaticMesh|SetStaticMesh (Variables|Default|GetStaticMesh) mesh)
  (Rendering|Material|SetVectorParameterValue (Variables|Default|GetmeshMaterial) "Color" Color :!class /Script/Engine.MaterialInstanceDynamic)
  (Rendering|Material|SetScalarParameterValue (Variables|Default|GetmeshMaterial) "EmmisiveAmount" EmmisiveAmount :!class /Script/Engine.MaterialInstanceDynamic))

(event EventBeginPlay
  (bind _returnvalue (Rendering|Material|CreateDynamicMaterialInstance (Variables|Default|GetStaticMesh) 0 "/Game/MaterialLibrary/M_3DIndicator_Inst.M_3DIndicator_Inst" "None" :!class /Script/Engine.PrimitiveComponent))
  (Variables|Default|SetmeshMaterial _returnvalue)
  (bind _returnvalue_2 (Rendering|Material|CreateDynamicMaterialInstance (Variables|Default|GetDecal) :!class /Script/Engine.DecalComponent))
  (Variables|Default|SetdecalMaterial _returnvalue_2))

(fn ConstructionScript)